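; BP_Wall is a map-kit wall that builds a back side from the mesh assigned to its front.
; Its construction script copies FrontMesh's static mesh to BackMesh and rotates it 180 degrees.
; It then offsets BackMesh along local Y to the front mesh's bounding-box minimum, so placement follows the chosen mesh's dimensions.
; The event graph holds only disabled placeholder events.
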(event EventBeginPlay)

(event Collision|EventActorBeginOverlap
  (params (OtherActor :type Actor%20Object%20Reference)))

(event EventTick
  (params (DeltaSeconds :type Float%20%28single-precision%29)))

(fn ConstructionScript
  (bind _backmesh (Variables|Default|GetBackMesh))
  (Components|StaticMesh|SetStaticMesh (Variables|Default|GetBackMesh) (Variables|/Script/Engine.StaticMeshComponent|GetStaticMesh (Variables|Default|GetFrontMesh)))
  (Transformation|SetRelativeRotation _backmesh "0,180.000000, 0" false false)
  (Transformation|SetRelativeLocation _backmesh (Math|Vector|MakeVector 0.0 (.Y (Math|Vector|BreakVector (.Min (Utilities|Struct|BreakBox (StaticMesh|GetBoundingBox (Variables|/Script/Engine.StaticMeshComponent|GetStaticMesh (Variables|Default|GetFrontMesh))))))) 0.0) false false))