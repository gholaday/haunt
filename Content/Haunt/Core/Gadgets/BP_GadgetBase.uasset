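; Base Blueprint for Haunt gadgets, handling pickup, drop, equip and unequip through an equipped flag on a single mesh.
; Drop enables physics and collision, restores the default material and throws the mesh along its relative forward vector.
; Pickup stops physics but leaves collision unchanged, as its NoCollision node is disconnected, while equip and unequip toggle visibility.
; Clipping events swap between first-person and default materials.
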(event Custom|EnableClippingMaterial
  (Rendering|Material|SetMaterial (Variables|Default|GetMesh) 0 (Variables|Default|GetFirstPersonMaterial)))

(event Custom|DisableClippingMaterial
  (Rendering|Material|SetMaterial (Variables|Default|GetMesh) 0 (Variables|Default|GetDefaultMaterial)))

(event EventBeginPlay)

(event Collision|EventActorBeginOverlap
  (params (OtherActor :type Actor%20Object%20Reference)))

(event EventTick
  (params (DeltaSeconds :type Float%20%28single-precision%29)))

(fn ConstructionScript)

(fn OnGadgetDrop
  (bind _mesh (Variables|Default|GetMesh))
  (Physics|SetSimulatePhysics _mesh true)
  (Collision|SetCollisionEnabled _mesh "QueryAndPhysics")
  (CallFunction|DisableClippingMaterial)
  (Physics|AddImpulse (Variables|Default|GetMesh) (* (Math|Vector|GetForwardVector (Variables|/Script/Engine.SceneComponent|GetRelativeRotation _mesh)) 2.5e+03) "None" false)
  (Variables|Default|SetIsEquipped false))

(fn OnGadgetPickup
  (Physics|SetSimulatePhysics (Variables|Default|GetMesh) false)
  (Variables|Default|SetIsEquipped true))

(fn OnEquipped
  (Variables|Default|SetIsEquipped true)
  (Rendering|SetVisibility (Variables|Default|GetMesh) true true))

(fn OnUnEquipped
  (Variables|Default|SetIsEquipped false)
  (Rendering|SetVisibility (Variables|Default|GetMesh) false true))