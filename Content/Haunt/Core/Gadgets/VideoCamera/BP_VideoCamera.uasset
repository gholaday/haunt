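; BP_VideoCamera is a video camera gadget that renders a live feed of its view into a texture.
; On BeginPlay it creates its own render target, stores it as FeedTextureTarget and assigns it to its SceneCapture component.
; While IsEnabled, Tick throttles manual CaptureScene calls through a Delay, using CameraFeedFPS directly as the wait in seconds rather than as a frame rate.
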(event EventBeginPlay
  (|CallParentFunction)
  (bind _returnvalue (Rendering|CreateRenderTarget2D 256 256 "RTF_RGBA16f"))
  (bind _output_get (Variables|Default|SetFeedTextureTarget _returnvalue))
  (Variables|/Script/Engine.SceneCaptureComponent2D|SetTextureTarget (Variables|Default|GetSceneCapture) _output_get))

(event EventTick
  (params (DeltaSeconds :type Float%20%28single-precision%29))
  (if (Variables|Default|GetIsEnabled)
    (Utilities|FlowControl|Delay (Variables|Default|GetCameraFeedFPS))
    (Rendering|SceneCapture|CaptureScene (Variables|Default|GetSceneCapture) :!class /Script/Engine.SceneCaptureComponent2D)))

(fn ConstructionScript
  (|CallParentFunction))