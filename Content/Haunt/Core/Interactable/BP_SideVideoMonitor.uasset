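; BP_SideVideoMonitor is an interactable side monitor that selects which camera feed the main video monitor uses.
; On interact, it finds BP_MainVideoMonitor with GetActorOfClass and copies its own CameraFeedIndex onto it.
; Alt-interact is empty, and the Blueprint has no other active logic.
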(event EventBeginPlay
  (|CallParentFunction) ; This node is disabled and will not be called.\nDrag off pins to build functionality.
)

(event Collision|EventActorBeginOverlap
  (params (OtherActor :type Actor%20Object%20Reference))
  (|CallParentFunction OtherActor) ; This node is disabled and will not be called.\nDrag off pins to build functionality.
)

(event EventTick
  (params (DeltaSeconds :type Float%20%28single-precision%29))
  (|CallParentFunction DeltaSeconds) ; This node is disabled and will not be called.\nDrag off pins to build functionality.
)

(event EventOnInteract
  (bind _returnvalue (Actor|GetActorOfClass "/Game/Haunt/Core/Interactable/BP_MainVideoMonitor.BP_MainVideoMonitor_C"))
  (Variables|/Game/Haunt/Core/Interactable/BP_MainVideoMonitor.BP_MainVideoMonitor_C|SetCameraFeedIndex _returnvalue (Variables|Default|GetCameraFeedIndex)))

(event EventOnAltInteract)

(fn ConstructionScript
  (|CallParentFunction))