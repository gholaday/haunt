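; BP_SideBodyCamVideoMonitor is an interactable side monitor for a player body cam feed, which switches the main video monitor to that feed on interaction.
; Shortly after BeginPlay it labels itself from CameraFeedID, replacing "p" with "Player".
; OnInteract finds BP_MainVideoMonitor and passes the ID to ChangeFeedServer.
; SetFeedTexture displays a supplied feed texture through a dynamic material instance on the screen.
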(event EventBeginPlay
  (Utilities|FlowControl|Delay 0.2)
  (CallFunction|SetCameraIndexText))

(event EventOnInteract
  (bind _returnvalue (Actor|GetActorOfClass "/Game/Haunt/Core/Interactable/BP_MainVideoMonitor.BP_MainVideoMonitor_C"))
  (Default|ChangeFeedServer _returnvalue (Variables|Default|GetCameraFeedID)))

(fn ConstructionScript
  (|CallParentFunction))

(fn SetCameraIndexText
  (bind _output_get (Variables|Default|SetDisplayText (Utilities|Text|ToText(String) (Utilities|String|Replace (Variables|Default|GetCameraFeedID) "p" "Player "))))
  (Rendering|Components|TextRender|SetText (Variables|Default|GetTextRender) _output_get))

(fn SetFeedTexture
  (params (FeedTexture :type Texture%20Render%20Target%202D%20Object%20Reference))
  (bind _screen (Variables|Default|GetScreen))
  (bind _returnvalue (Rendering|Material|CreateDynamicMaterialInstance _screen 0 "/Game/Haunt/Core/Gadgets/VideoCamera/CameraFeed_Mat.CameraFeed_Mat" "None" :!class /Script/Engine.PrimitiveComponent))
  (Rendering|Material|SetMaterial _screen 0 _returnvalue)
  (bind _output_get (Variables|Default|SetFeedTextureTarget FeedTexture))
  (Rendering|Material|SetTextureParameterValue _returnvalue "Tex" _output_get))