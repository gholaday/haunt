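; BP_MainVideoMonitor is an in-world monitor that displays a video camera's feed and label, starting on feed "0" shortly after BeginPlay.
; Server and Multi events switch feeds by ID, resolving cameras through GS_DefaultGameState.
; ChangeFeed applies the camera's render target to a dynamic screen material and updates the text.
; Tick, throttled by a Delay, shows static whenever the current camera is not both recording and enabled.
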(event Custom|ChangeFeed_Server
  (params (CameraFeedID :type String))
  (CallFunction|ChangeFeedMulti CameraFeedID))

(event Custom|ChangeFeed_Multi
  (params (CameraFeedID :type String))
  (bind _asgs_default_game_state (Utilities|Casting|CastToGS_DefaultGameState (Game|GetGameState)))
  (bind _videocameracomponent (Default|GetCameraFeedbyID _asgs_default_game_state CameraFeedID))
  (CallFunction|ChangeFeed _videocameracomponent))

(event EventTick
  (params (DeltaSeconds :type Float%20%28single-precision%29))
  (bind _video_camera_component (Variables|Default|GetVideo%20Camera%20Component))
  (Utilities|FlowControl|Delay 0.1)
  (Utilities|IsValid _video_camera_component
    (:Is%20Valid
      (Rendering|SetVisibility (Variables|Default|GetStatic) (not (and (Variables|/Game/Haunt/Core/Engine/VideoCameraComponent.VideoCameraComponent_C|GetIsRecording _video_camera_component) (Variables|/Game/Haunt/Core/Engine/VideoCameraComponent.VideoCameraComponent_C|GetIsEnabled _video_camera_component))) false))))

(event EventBeginPlay
  (Utilities|FlowControl|Delay 0.5)
  (bind _asgs_default_game_state (Utilities|Casting|CastToGS_DefaultGameState (Game|GetGameState)))
  (bind _videocameracomponent (Default|GetCameraFeedbyID _asgs_default_game_state "0"))
  (CallFunction|ChangeFeed _videocameracomponent))

(fn ConstructionScript)

(fn ChangeFeed
  (params (VideoCameraComponent :type Video%20Camera%20Component%20Object%20Reference))
  (bind _screen (Variables|Default|GetScreen))
  (Utilities|IsValid VideoCameraComponent
    (:Is%20Valid
      (bind _output_get (Variables|Default|SetVideo%20Camera%20Component VideoCameraComponent))
      (Rendering|Components|TextRender|SetText (Variables|Default|GetTextRender) (Utilities|Text|ToText(String) (Variables|/Game/Haunt/Core/Engine/VideoCameraComponent.VideoCameraComponent_C|GetDisplayText _output_get)))
      (bind _returnvalue (Rendering|Material|CreateDynamicMaterialInstance _screen 0 "/Game/Haunt/Core/Gadgets/VideoCamera/CameraFeed_Mat.CameraFeed_Mat" "None" :!class /Script/Engine.PrimitiveComponent))
      (Rendering|Material|SetMaterial _screen 0 _returnvalue)
      (Rendering|Material|SetTextureParameterValue _returnvalue "Tex" (Variables|/Game/Haunt/Core/Engine/VideoCameraComponent.VideoCameraComponent_C|GetFeedTextureTarget _output_get)))))