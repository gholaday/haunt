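; Interactable light switch actor that turns a circuit of lights on and off.
; OnInteract calls ToggleLights, which flips the visibility of each light component in LightsInCircuit.
; The construction script flushes persistent debug lines, then redraws switch-to-light lines for every switch instance with ShowDebugLines enabled, visualizing the circuit wiring.
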(event EventBeginPlay)

(event Collision|EventActorBeginOverlap
  (params (OtherActor :type Actor%20Object%20Reference)))

(event EventTick
  (params (DeltaSeconds :type Float%20%28single-precision%29)))

(event EventOnInteract
  (CallFunction|ToggleLights))

(fn ConstructionScript
  (CallFunction|DrawDebugLines))

(fn DrawDebugLines
  (Rendering|Debug|FlushPersistentDebugLines)
  (bind _outactors (Actor|GetAllActorsOfClass "BP_Lightswitch_Component_C"))
  (for _array_element _outactors
    (if (Variables|BP_Lightswitch_Component_C|GetShowDebugLines _array_element)
      (for _array_element_2 (Variables|BP_Lightswitch_Component_C|GetLightsInCircuit _array_element)
        (Rendering|Debug|DrawDebugLine (Transformation|GetWorldLocation (Variables|BP_Lightswitch_Component_C|GetDefaultSceneRoot _array_element)) (Transformation|GetWorldLocation (Variables|/Script/Engine.Light|GetLightComponent _array_element_2)) "(R=0.035845,G=0.000000,B=0.994792,A=1.000000)" 9999.0 1.0)))))

(fn ToggleLights
  (for _array_element (Variables|Default|GetLightsInCircuit)
    (Rendering|ToggleVisibility (Variables|/Script/Engine.Light|GetLightComponent _array_element) false)))