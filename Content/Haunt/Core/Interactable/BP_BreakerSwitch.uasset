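; BP_BreakerSwitch is an interactable breaker that reports whether it gives power, meaning turned on and not broken.
; Interacting toggles it and recolors an indicator green or red through a dynamic material created in the construction script.
; Tick forces it off while broken without refreshing the indicator color.
; RegisterSwitch adds light switches to a list and returns the breaker itself, but nothing here notifies them of changes.
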(event EventBeginPlay
  (|CallParentFunction) ; This node is disabled and will not be called.\nDrag off pins to build functionality.
)

(event Collision|EventActorBeginOverlap
  (params (OtherActor :type Actor%20Object%20Reference))
  (|CallParentFunction OtherActor) ; This node is disabled and will not be called.\nDrag off pins to build functionality.
)

(event EventTick
  (params (DeltaSeconds :type Float%20%28single-precision%29))
  (|CallParentFunction DeltaSeconds)
  (if (Variables|Default|GetIsBroken)
    (Variables|Default|SetIsTurnedOn false)))

(event EventOnInteract
  (Variables|Default|SetIsTurnedOn (not (Variables|Default|GetIsTurnedOn)))
  (CallFunction|ColorIndicator))

(fn ConstructionScript
  (|CallParentFunction)
  (bind _returnvalue (Rendering|Material|CreateDynamicMaterialInstance (Rendering|Material|GetMaterial (Variables|Default|GetIndicator) 0) "None" "Transient" :!class /Script/Engine.KismetMaterialLibrary))
  (Rendering|Material|SetMaterial (Variables|Default|GetIndicator) 0 _returnvalue)
  (Variables|Default|SetIndicatorMID _returnvalue)
  (CallFunction|ColorIndicator))

(fn IsGivingPower
  (return (and (Variables|Default|GetIsTurnedOn) (not (Variables|Default|GetIsBroken)))))

(fn RegisterSwitch
  (params (Switch :type BP%20Lightswitch%20Component%20Object%20Reference))
  (Utilities|Array|Add (Variables|Default|GetLightSwitches) Switch)
  (return self))

(fn ColorIndicator
  (bind _indicatormid (Variables|Default|GetIndicatorMID))
  (bind _isgivingpower (CallFunction|IsGivingPower))
  (Utilities|IsValid (Variables|Default|GetIndicatorMID)
    (:Is%20Valid
      (if _isgivingpower
        (Rendering|Material|SetVectorParameterValue _indicatormid "Color" "(R=0.000000,G=0.562500,B=0.102771,A=1.000000)" :!class /Script/Engine.MaterialInstanceDynamic)
        (else
          (Rendering|Material|SetVectorParameterValue _indicatormid "Color" "(R=0.265625,G=0.000000,B=0.031221,A=1.000000)" :!class /Script/Engine.MaterialInstanceDynamic))))))