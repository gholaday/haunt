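; Player character Blueprint for Haunt, providing a toggleable flashlight, stamina-limited sprinting and crouching.
; Tick runs EnergyRegen, which drains Stamina while sprinting, calls StopSprinting once it drops below zero, and otherwise recharges it toward a fixed cap.
; Sprint functions swap the movement component's max walk speed, with starting blocked while crouched.
; Crouch functions wrap the built-in Crouch and UnCrouch, starting only on the ground.
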(event Custom|ToggleFlashlight
  ;[1 1 1] Flashlight
  (bind _output_get (Variables|Default|SetIsFlashlightOn (not (Variables|Default|GetIsFlashlightOn))))
  (Rendering|SetVisibility (Variables|Default|GetSpotLight) _output_get true))

(event EventTick
  (params (DeltaSeconds :type Float%20%28single-precision%29))
  (CallFunction|EnergyRegen DeltaSeconds))

(event Collision|EventActorBeginOverlap
  (params (OtherActor :type Actor%20Object%20Reference)))

(event EventBeginPlay)

(fn ConstructionScript)

(fn StartSprinting
  (if (>= (Variables|Locomotion|GetStamina) 0.0)
    (if (not (Variables|Default|GetbIsCrouched))
      (Variables|Locomotion|SetIsSprinting true)
      (Variables|/Script/Engine.CharacterMovementComponent|SetMaxWalkSpeed (Variables|Character|GetCharacterMovement) (Variables|Locomotion|GetSprintSpeed)))))

(fn StopSprinting
  (Variables|Locomotion|SetIsSprinting false)
  (Variables|/Script/Engine.CharacterMovementComponent|SetMaxWalkSpeed (Variables|Character|GetCharacterMovement) (Variables|Locomotion|GetWalkSpeed)))

(fn EnergyRegen
  (params (DeltaTime :type Float%20%28single-precision%29))
  (if (Variables|Locomotion|GetIsSprinting)
    (if (>= (Variables|Locomotion|GetStamina) 0.0)
      (Variables|Locomotion|SetStamina (- (Variables|Locomotion|GetStamina) (* DeltaTime (Variables|Locomotion|GetStaminaDepletionRate))))
      (else
        (CallFunction|StopSprinting)))
    (elif (not (>= (Variables|Locomotion|GetStamina) 1e+02))
      (Variables|Locomotion|SetStamina (+ (* DeltaTime (Variables|Locomotion|GetStaminaRechargeRate)) (Variables|Locomotion|GetStamina))))))

(fn StartCrouching
  (if (AI|Components|NavMovement|IsMovingonGround (Variables|Character|GetCharacterMovement))
    (Character|Crouch)))

(fn StopCrouching
  (Character|UnCrouch))