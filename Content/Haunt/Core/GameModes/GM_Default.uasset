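; Default game mode for a ghost-haunting game, tracking the player team's average sanity and showing FPS stats from BeginPlay.
; Tick uses a one-second Delay as a throttle, then on authority averages all BP_Player sanity values, floors the result and prints it.
; AssignTeams is an empty stub, and the IsGhostInHauntPhase OnRep does nothing because its light-flicker logic is disconnected.
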(event EventBeginPlay
  (Development|ExecuteConsoleCommand "stat fps" 0))

(event EventTick
  (params (DeltaSeconds :type Float%20%28single-precision%29))
  (Utilities|FlowControl|Delay 1.0)
  (Networking|SwitchHasAuthority
    (:Authority
      (Utilities|GetPlayerTeamAverageSanity))))

(fn ConstructionScript)

(fn AssignTeams)

(fn OnRepIsGhostinHauntPhase)