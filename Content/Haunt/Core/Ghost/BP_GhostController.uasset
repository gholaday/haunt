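; AI controller for the ghost that runs BT_Ghost and feeds it a target enemy and a visibility flag.
; After a short delay on BeginPlay, it caches all BP_Player actors as enemies and starts the tree.
; Perception updates, also delayed, write the visibility key from each actor's first last-sensed stimulus, even for non-enemies.
; Actors found in the enemy list also become the blackboard target.
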(event EventBeginPlay
  (Utilities|FlowControl|Delay 3.0)
  (CallFunction|SetEnemies)
  (AI|RunBehaviorTree "/Game/Haunt/Core/Ghost/BehaviorTrees/BT_Ghost.BT_Ghost"))

(event EventTick
  (params (DeltaSeconds :type Float%20%28single-precision%29)))

(event OnPerceptionUpdated(AIPerception)
  (params (UpdatedActors :type Array%20of%20Actor%20Object%20References))
  (Utilities|FlowControl|Delay 3.0)
  (for _array_element UpdatedActors
    (CallFunction|UpdateBlackboardKeys (Variables|Default|GetAIPerception) _array_element)
    (CallFunction|SetTargetEnemy _array_element)))

(event OnTargetPerceptionUpdated(AIPerception)
  (params (Actor :type Actor%20Object%20Reference) (Stimulus :type AI%20Stimulus%20Structure))
  (if (.bSuccessfullySensed (Utilities|Struct|BreakAIStimulus Stimulus))
    _))

(fn ConstructionScript)

(fn SetEnemies
  (bind _outactors (Actor|GetAllActorsOfClass "/Game/Haunt/Core/Player/BP_Player.BP_Player_C"))
  (for _array_element _outactors
    (Utilities|Array|Add (Variables|Default|GetEnemies) _array_element)))

(fn SetTargetEnemy
  (params (NewTarget :type Actor%20Object%20Reference))
  (if (Utilities|Array|ContainsItem (Variables|Default|GetEnemies) NewTarget)
    (bind _output_get (Variables|Default|SetTargetEnemy NewTarget))
    (AI|Components|Blackboard|SetValueasObject (AI|GetBlackboard 0) (Utilities|Name|MakeLiteralName "BBKTargetEnemy") _output_get)
    (CallFunction|UpdateBlackboardKeys (Variables|Default|GetAIPerception) (Variables|Default|GetTargetEnemy))))

(fn UpdateBlackboardKeys
  (params (PerceptionComponent :type AI%20Perception%20Component%20Object%20Reference) (EnemyActor :type Actor%20Object%20Reference))
  (bind _info (Class|AIPerceptionComponent|GetActorsPerception PerceptionComponent EnemyActor))
  (AI|Components|Blackboard|SetValueasBool (AI|GetBlackboard 0) (Utilities|Name|MakeLiteralName "BBKIsEnemyVisible") (.bSuccessfullySensed (Utilities|Struct|BreakAIStimulus (Utilities|Array|Get(acopy) (.LastSensedStimuli (Utilities|Struct|BreakActorPerceptionBlueprintInfo _info)))))))